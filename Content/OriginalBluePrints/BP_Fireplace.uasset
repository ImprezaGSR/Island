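; Interactable fireplace that the player lights and puts out, acting as a heat source for BP_ThirdPersonCharacter.
; Interact flip-flops the fire particle and prompt text, while looking at or away from the fireplace shows or hides the prompt widget.
; SenseHeatRange adds or removes itself from the overlapping character's HotObjects, and is scaled to zero while unlit instead of toggling overlap events.
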(event `self.ReceiveBeginPlay`
  (bind _senseheatrange (`self.SenseHeatRange`))
  (bind _asinteractive_prompt_w (cast `/Game/OriginalBluePrints/InteractivePrompt_W` (`WidgetComponent.GetUserWidgetObject` (`self.Widget`))))
  (`/Game/OriginalBluePrints/InteractivePrompt_W.SetText` _asinteractive_prompt_w "Press 'Right Click' to Start Fire")
  (set `self.HeatRangeScale` (`SceneComponent.RelativeScale3D` _senseheatrange))
  (if (not (`self.isFireLit`))
    (`SceneComponent.SetRelativeScale3D` _senseheatrange (0.0 0.0 0.0))))

(event `AddFireEffect`
  (bind _senseheatrange (`self.SenseHeatRange`))
  (bind _returnvalue (`WidgetComponent.GetUserWidgetObject` (`self.Widget`)))
  (`/Engine/EditorBlueprintResources/StandardMacros.FlipFlop`
    (:`A`
      (bind _fireparticle (`self.FireParticle`)
        (:`then`
          (`ActorComponent.Activate` _fireparticle false))
        (:`else`
          (bind _returnvalue_2 (`GameplayStatics.SpawnEmitterAtLocation` "/Game/StarterContent/Particles/P_Fire.P_Fire" (`self.K2_GetActorLocation`) (struct) (2.0 2.0 2.0)))
          (set `self.FireParticle` _returnvalue_2)))
      (set `self.isFireLit` true)
      (set `self.isFireHasLit` true)
      (bind _asinteractive_prompt_w (cast `/Game/OriginalBluePrints/InteractivePrompt_W` _returnvalue))
      (`/Game/OriginalBluePrints/InteractivePrompt_W.SetText` _asinteractive_prompt_w "Press 'Right Click' to Stop Fire")
      (`SceneComponent.SetRelativeScale3D` _senseheatrange (`self.HeatRangeScale`)))
    (:`B`
      (`ActorComponent.Deactivate` (`self.FireParticle`))
      (set `self.isFireLit` false)
      (bind _asinteractive_prompt_w_2 (cast `/Game/OriginalBluePrints/InteractivePrompt_W` _returnvalue))
      (`/Game/OriginalBluePrints/InteractivePrompt_W.SetText` _asinteractive_prompt_w_2 "Press 'Right Click' to Start Fire")
      (`SceneComponent.SetRelativeScale3D` _senseheatrange (0.0 0.0 0.0)))))

(event `ShowPrompt`
  (`SceneComponent.SetHiddenInGame` (`self.Widget`) false false))

(event `HidePrompt`
  (`SceneComponent.SetHiddenInGame` (`self.Widget`) true false))

(event `self.SenseHeatRange.OnComponentBeginOverlap`
  (params (OverlappedComponent :type "PrimitiveComponent Object Reference") (OtherActor :type "Actor Object Reference") (OtherComp :type "PrimitiveComponent Object Reference") (OtherBodyIndex :type Integer) (bFromSweep :type Boolean) (SweepResult :type "HitResult Structure (by ref)"))
  (bind _asbp_third_person_character (cast `/Game/ThirdPerson/Blueprints/BP_ThirdPersonCharacter` OtherActor))
  (`KismetArrayLibrary.Array_Add` (`/Game/ThirdPerson/Blueprints/BP_ThirdPersonCharacter.hotObjects` _asbp_third_person_character) (`self.SenseHeatRange`)))

(event `self.SenseHeatRange.OnComponentEndOverlap`
  (params (OverlappedComponent :type "PrimitiveComponent Object Reference") (OtherActor :type "Actor Object Reference") (OtherComp :type "PrimitiveComponent Object Reference") (OtherBodyIndex :type Integer))
  (bind _asbp_third_person_character (cast `/Game/ThirdPerson/Blueprints/BP_ThirdPersonCharacter` OtherActor))
  (`KismetArrayLibrary.Array_RemoveItem` (`/Game/ThirdPerson/Blueprints/BP_ThirdPersonCharacter.hotObjects` _asbp_third_person_character) (`self.SenseHeatRange`)))

(fn `Interact`
  (params (Interactor :type "Character Object Reference") (key :type "Key Structure"))
  (returns (`Success?` :type Boolean))
  (`self.AddFireEffect`)
  (return true))

(fn `InteractReleased`
  (params (Interactor :type "Character Object Reference") (key :type "Key Structure"))
  (returns (`Success?` :type Boolean))
  (return false))

(fn `LookingAtObject`
  (params (Interactor :type "Character Object Reference"))
  (returns (`Success?` :type Boolean))
  (`self.ShowPrompt`)
  (return true))

(fn `NotLookingAtObject`
  (params (Interactor :type "Character Object Reference"))
  (returns (`Success?` :type Boolean))
  (`self.HidePrompt`)
  (return true))

(fn `UserConstructionScript`)