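; BP_Quest is the base actor for quests in the quest system, owning a root objective collection that it exposes through a getter.
; On BeginPlay it builds the root collection, populates it with objectives and activates it.
; The construct and populate functions are placeholders that print an error, so child quest Blueprints are expected to override them to define their objectives.
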(event `self.ReceiveBeginPlay`
  (bind _rootobjcollection (`self.ConstructNewObjectiveCollection`))
  (bind _output_get (set `self.RootObjectiveCollection` _rootobjcollection))
  (`self.PopulateObjectives` _output_get)
  (`/Game/QuestSystem/ObjectiveClasses/BP_Objective.ActivateObjective` (`self.RootObjectiveCollection`)))

(fn `ConstructNewObjectiveCollection`
  (returns (RootObjCollection :type "/Game/QuestSystem/ObjectiveClasses/BP_ObjCollection Object Reference"))
  (`KismetSystemLibrary.PrintString` "Error: ConstructNewObjectiveCollection called for base class!")
  (return null))

(fn `GetRootObjectiveCollection`
  (returns (RootObjectiveCollection :type "/Game/QuestSystem/ObjectiveClasses/BP_Objective Object Reference"))
  (return (`self.RootObjectiveCollection`)))

(fn `PopulateObjectives`
  (params (RootObjCollection :type "/Game/QuestSystem/ObjectiveClasses/BP_ObjCollection Object Reference"))
  (`KismetSystemLibrary.PrintString` "Error: PopulateObjective called for base class!"))

(fn `UserConstructionScript`)