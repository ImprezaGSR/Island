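; BP_QuestTraitor is a quest titled "As a Traitor" that defines a single objective to kill a Dummy.
; ConstructNewObjectiveCollection creates the root objective collection with no required order.
; PopulateObjectives constructs a kill-characters objective from the Dummy variable and adds it to that collection.
; The event graph and construction script add no logic of their own.
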(fn `ConstructNewObjectiveCollection`
  (returns (RootObjCollection :type "/Game/QuestSystem/ObjectiveClasses/BP_ObjCollection Object Reference"))
  (bind _returnvalue (`|GenericCreateObject` "/Game/QuestSystem/ObjectiveClasses/BP_ObjCollection.BP_ObjCollection_C" false "As a Traitor"))
  (return _returnvalue))

(fn `PopulateObjectives`
  (params (RootObjCollection :type "/Game/QuestSystem/ObjectiveClasses/BP_ObjCollection Object Reference"))
  (bind _returnvalue (`|GenericCreateObject` "/Game/QuestSystem/ObjectiveClasses/BP_ObjKillCharacters.BP_ObjKillCharacters_C" (`self.Dummy`) "Kill a Dummy"))
  (`/Game/QuestSystem/ObjectiveClasses/BP_ObjCollection.AddObjective` (`local.RootObjCollection`) _returnvalue))

(fn `UserConstructionScript`
  (`parent.UserConstructionScript`))