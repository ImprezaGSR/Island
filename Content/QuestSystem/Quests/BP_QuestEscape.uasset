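; BP_QuestEscape is a quest definition for escaping the island, built from objective objects.
; It overrides the root collection factory to create an unordered BP_ObjCollection named for the escape goal.
; PopulateObjectives then constructs reach-destination objectives bound to the red, blue and green marker triggers and adds them to that collection, so they can be completed in any order.
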(fn `ConstructNewObjectiveCollection`
  (returns (RootObjCollection :type "/Game/QuestSystem/ObjectiveClasses/BP_ObjCollection Object Reference"))
  (bind _returnvalue (`|GenericCreateObject` "/Game/QuestSystem/ObjectiveClasses/BP_ObjCollection.BP_ObjCollection_C" false "To Escape from the Island"))
  (return _returnvalue))

(fn `PopulateObjectives`
  (params (RootObjCollection :type "/Game/QuestSystem/ObjectiveClasses/BP_ObjCollection Object Reference"))
  (`|ExecutionSequence`
    (:`then_0`
      (bind _returnvalue (`|GenericCreateObject` "/Game/QuestSystem/ObjectiveClasses/BP_ObjReachDestination.BP_ObjReachDestination_C" (`self.RedMarkerTrigger`) "Reach Red Marker"))
      (`/Game/QuestSystem/ObjectiveClasses/BP_ObjCollection.AddObjective` (`local.RootObjCollection`) _returnvalue))
    (:`then_1`
      (bind _returnvalue_2 (`|GenericCreateObject` "/Game/QuestSystem/ObjectiveClasses/BP_ObjReachDestination.BP_ObjReachDestination_C" (`self.Blue Marker Trigger`) "Reach Blue Marker"))
      (`/Game/QuestSystem/ObjectiveClasses/BP_ObjCollection.AddObjective` (`local.RootObjCollection`) _returnvalue_2))
    (:`then_2`
      (bind _returnvalue_3 (`|GenericCreateObject` "/Game/QuestSystem/ObjectiveClasses/BP_ObjReachDestination.BP_ObjReachDestination_C" (`self.GreenMarkerTrigger`) "Reach Green Marker"))
      (`/Game/QuestSystem/ObjectiveClasses/BP_ObjCollection.AddObjective` (`local.RootObjCollection`) _returnvalue_3))))

(fn `UserConstructionScript`
  (`parent.UserConstructionScript`))